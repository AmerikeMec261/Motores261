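; Overworld wolf enemy that patrols and starts a battle when it reaches the player.
; It wanders to random reachable points; PawnSensing triggers a faster chase, with a retriggerable delay resuming patrol.
; Reaching the player fires ArriveToPlayer, bound to BeginFigth, which calls Rakhi_BP's TeleportToFigth and records the spawn name as defeated in the GameInstance.
; Separately, capsule overlap with a Player-tagged actor opens a level directly.
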(event OnComponentBeginOverlap(CapsuleComponent)
  (params (OverlappedComponent :type Primitive%20Component%20Object%20Reference) (OtherActor :type Actor%20Object%20Reference) (OtherComp :type Primitive%20Component%20Object%20Reference) (OtherBodyIndex :type Integer) (bFromSweep :type Boolean) (SweepResult :type Hit%20Result%20Structure%20%28by%20ref%29))
  (if (Actor|ActorHasTag OtherActor "Player")
    (Game|OpenLevel(byObjectReference) (Variables|Default|GetLevel))))

(event OnSeePawn(PawnSensing)
  (params (Pawn :type Pawn%20Object%20Reference))
  ;[1 1 1] Ver
  ;[1 1 1] Ir hacia Jugador
  (Utilities|FlowControl|Sequence
    (:then_0
      (Variables|/Script/Engine.CharacterMovementComponent|SetMaxWalkSpeed (Variables|Character|GetCharacterMovement) 8e+02)
      (AI|AIMoveTo self "0, 0, 0" (Game|GetPlayerCharacter 0) 1e+02 false
        (:OnSuccess
          ;[1 1 1] Detecta que tocó al jugador
          (Default|CallArrivetoPlayer)
          (Development|PrintString "tocoplayer"))))
    (:then_1
      (Utilities|FlowControl|RetriggerableDelay 5.0)
      (CallFunction|Patrullando))))

(event Custom|BeginFigth
  (bind _nombrespawn (Variables|Default|GetNombreSpawn))
  ;[1 1 1] Comenzar Batalla
  (bind _asrakhi_bp (Utilities|Casting|CastToRakhi_BP (Game|GetPlayerCharacter 0)))
  (Default|TeleporttoFigth _asrakhi_bp self (Variables|Default|GetNumberOfEnemiesToSpawn))
  (bind _asbp_game_instance (Utilities|Casting|CastToBP_GameInstance (Game|GetGameInstance)))
  (Development|PrintString _nombrespawn true true "(R=0.000000,G=0.660000,B=1.000000,A=1.000000)" 2e+01)
  (Utilities|Array|Add (Variables|/Game/Rakhi/Cerebro_De_Juego/BP_GameInstance.BP_GameInstance_C|GetEnemigosDerrotados _asbp_game_instance) _nombrespawn))

(event Custom|Patrullando
  ;[1 1 1] Patrullaje
  (EventDispatchers|BindEventtoArrivetoPlayer (delegate Custom|BeginFigth))
  (AI|AIMoveTo self (.RandomLocation (AI|Navigation|GetRandomReachablePointinRadius (Transformation|GetWorldLocation (Variables|Default|GetSprite)) 1.5e+03 0 0)) 0 5.0 false
    (:OnSuccess
      (Utilities|FlowControl|Delay 2.0)
      (CallFunction|Patrullando))
    (:OnFail
      (Utilities|FlowControl|Delay 5.0)
      (CallFunction|Patrullando))))

(event EventBeginPlay
  (CallFunction|Patrullando))

(fn ConstructionScript)