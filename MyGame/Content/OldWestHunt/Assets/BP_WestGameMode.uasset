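; BP_WestGameMode is the game mode for OldWestHunt, providing helper functions that update player score and ammo stored in BPGI_GameInstance.
; AddToScore adds to the clamped score, while AddToBullets and WasteBullets raise or lower a small clamped bullet count and print it for debugging.
; Bullet functions share a CastToGameInstance helper; AddToVulturesHit is an empty stub, and the event graph has no active logic.
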(event EventBeginPlay)

(event EventTick
  (params (DeltaSeconds :type Float%20%28single-precision%29)))

(fn ConstructionScript)

(fn AddtoScore
  (params (ScoreToAdd :type Float%20%28double-precision%29))
  (bind _asbpgi_game_instance (Utilities|Casting|CastToBPGI_GameInstance (Game|GetGameInstance)))
  (Variables|/Game/OldWestHunt/Assets/BPGI_GameInstance.BPGI_GameInstance_C|SetScore _asbpgi_game_instance (Math|Float|Clamp(Float) (+ ScoreToAdd (Variables|/Game/OldWestHunt/Assets/BPGI_GameInstance.BPGI_GameInstance_C|GetScore _asbpgi_game_instance)) 0.0 1e+05)))

(fn AddtoBullets
  (params (B :type Integer) (Objetivo :type BP%20UI%20Object%20Reference))
  (bind _asbpgi_game_instance (CallFunction|CasttoGameInstance))
  (bind _output_get (Variables|/Game/OldWestHunt/Assets/BPGI_GameInstance.BPGI_GameInstance_C|SetBullets _asbpgi_game_instance (Math|Integer|Clamp(Integer) (+ (Variables|/Game/OldWestHunt/Assets/BPGI_GameInstance.BPGI_GameInstance_C|GetBullets _asbpgi_game_instance) B) 0 3)))
  (Development|PrintString (Utilities|String|ToString(Integer) _output_get)))

(fn AddtoVulturesHit)

(fn CasttoGameInstance
  (bind _asbpgi_game_instance (Utilities|Casting|CastToBPGI_GameInstance (Game|GetGameInstance)))
  (return _asbpgi_game_instance))

(fn WasteBullets
  (params (B :type Integer) (Objetivo :type BP%20UI%20Object%20Reference))
  (bind _asbpgi_game_instance (CallFunction|CasttoGameInstance))
  (bind _output_get (Variables|/Game/OldWestHunt/Assets/BPGI_GameInstance.BPGI_GameInstance_C|SetBullets _asbpgi_game_instance (Math|Integer|Clamp(Integer) (- (Variables|/Game/OldWestHunt/Assets/BPGI_GameInstance.BPGI_GameInstance_C|GetBullets _asbpgi_game_instance) B) 0 3)))
  (Development|PrintString (Utilities|String|ToString(Integer) _output_get)))