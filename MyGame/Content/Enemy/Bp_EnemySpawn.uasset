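; Enemy spawn point that places a touch enemy in the level unless that enemy has already been defeated.
; On BeginPlay it asks GameMode_Rakhi whether the enemy with its configured name is defeated and prints the result for debugging.
; If defeated it destroys itself; otherwise it spawns one Bp_EnemyCharacterTouch at its transform and passes the name to it as NombreSpawn.
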(event EventBeginPlay
  (bind _nombredelenemigo (Variables|Default|GetNombreDelEnemigo))
  (bind _asgame_mode_rakhi (Utilities|Casting|CastToGameMode_Rakhi (Game|GetGameMode)))
  (bind _estaderrotado (Default|ReadEstaDerrotado? _asgame_mode_rakhi _nombredelenemigo))
  (Development|PrintString (Utilities|String|Append "Esta derrotado: " (Utilities|String|ToString(Boolean) _estaderrotado) _nombredelenemigo) true true "(R=0.000000,G=0.660000,B=1.000000,A=1.000000)" 1e+01)
  (if _estaderrotado
    (Actor|DestroyActor)
    (else
      (for _index (range 0 0)
        (bind _returnvalue (Game|SpawnActorfromClass "/Game/Enemy/Bp_EnemyCharacterTouch.Bp_EnemyCharacterTouch_C" (Transformation|GetActorTransform) "Undefined" "MultiplyWithRoot" 0 0))
        (Variables|/Game/Enemy/Bp_EnemyCharacterTouch.Bp_EnemyCharacterTouch_C|SetNombreSpawn _returnvalue (Variables|Default|GetNombreDelEnemigo))))))

(fn ConstructionScript)