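; Player controller that opens the pause menu and holds helpers for creating UI widgets.
; The AI_Inventario input pauses the game, shows the cursor and adds WB_Menu_Pausa, while BeginPlay creates and stores a player HUD widget without adding it to the viewport.
; An inventory toggle, which feeds the player's BPC_Inventory into WB_InventoryUI, is disconnected.
; DisplayMainMenu is never called here and discards its created widget, setting WBMenu to None.
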(event Input|EnhancedActionEvents|EnhancedInputActionAI_Inventario
  (params (ActionValue :type Boolean) (ElapsedSeconds :type Float%20%28double-precision%29) (TriggeredSeconds :type Float%20%28double-precision%29) (InputAction :type Input%20Action%20Object%20Reference :default "/Game/Inventario/AI_Inventario.AI_Inventario"))
  (:Started
    (Game|SetGamePaused true)
    (Variables|Default|SetbShowMouseCursor true)
    (bind _returnvalue (UserInterface|CreateWidget "/Game/Ui/Pausa/WB_Menu_Pausa.WB_Menu_Pausa_C"))
    (UserInterface|Viewport|AddtoViewport _returnvalue 0)))

(event EventBeginPlay
  (CallFunction|DisplayPlayerHud))

(event EventTick
  (params (DeltaSeconds :type Float%20%28single-precision%29)))

(fn ConstructionScript)

(fn DisplayPlayerHud
  (bind _returnvalue (UserInterface|CreateWidget "/Game/Conversaciones/WBP_Conv_Player.WBP_Conv_Player_C"))
  (Variables|Default|SetWBP_Conv_Player _returnvalue))

(fn DisplayInventoryUi
  (bind _returnvalue (Game|GetPlayerCharacter 0))
  (bind _returnvalue_2 (Actor|GetComponentbyClass _returnvalue "/Game/Inventario/BPC_Inventory.BPC_Inventory_C"))
  (Utilities|IsValid _returnvalue_2
    (:Is%20Valid
      (bind _returnvalue_3 (UserInterface|CreateWidget "/Game/Inventario/UI/WB_InventoryUI.WB_InventoryUI_C" 0 _returnvalue_2))
      (bind _output_get (Variables|Default|SetWB_InventoryUI _returnvalue_3))
      (UserInterface|Viewport|AddtoViewport _output_get 0))))

(fn DisplayMainMenu
  (UserInterface|CreateWidget "/Game/Widgets/MainMenu/WBP_MainMenu.WBP_MainMenu_C")
  (bind _output_get (Variables|Default|SetWB_Menu 0))
  (UserInterface|Viewport|AddtoViewport _output_get 0))