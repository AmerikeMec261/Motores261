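; Enemy actor for a fight that moves toward the player, takes damage and sends the player back when defeated.
; On BeginPlay it runs AIMoveTo with the player controller as target and calls ArriveToPlayer on success.
; Damage arrives through an interface event, lowers life and refreshes the widget-component healthbar.
; At zero life it destroys itself and calls TeleportToBack on Rakhi_BP; capsule overlap with the player only prints.
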(event OnComponentBeginOverlap(CapsuleComponent)
  (params (OverlappedComponent :type Primitive%20Component%20Object%20Reference) (OtherActor :type Actor%20Object%20Reference) (OtherComp :type Primitive%20Component%20Object%20Reference) (OtherBodyIndex :type Integer) (bFromSweep :type Boolean) (SweepResult :type Hit%20Result%20Structure%20%28by%20ref%29))
  (if (Actor|ActorHasTag OtherActor "Player")
    (Development|PrintString "Toco al player")))

(event EventBeginPlay
  (AI|AIMoveTo self "0, 0, 0" (Game|GetPlayerController 0) 1e+02 false
    (:OnSuccess
      (Default|CallArrivetoPlayer)
      (Development|PrintString "tocoplayer"))))

(event Collision|EventActorBeginOverlap
  (params (OtherActor :type Actor%20Object%20Reference)))

(event EventTick
  (params (DeltaSeconds :type Float%20%28single-precision%29)))

(event EventIReceiveDamage
  (params (Damage :type Float%20%28double-precision%29))
  (CallFunction|ReceiveDamage Damage))

(fn ConstructionScript)

(fn ReceiveDamage
  (params (DamageToReceive :type Float%20%28double-precision%29))
  (bind _aswb_enemy_healthbar (Utilities|Casting|CastToWb_EnemyHealthbar (UserInterface|GetUserWidgetObject (Variables|Default|GetEnemyHealthbarWidget))))
  (bind _output_get (Variables|Default|SetCurrentLife (- (Variables|Default|GetCurrentLife) DamageToReceive)))
  (Default|UpdateHealthbar _aswb_enemy_healthbar _output_get (Variables|Default|GetMaxLife))
  (if (<= (Variables|Default|GetCurrentLife) 0.0)
    (Actor|DestroyActor)
    (bind _asrakhi_bp (Utilities|Casting|CastToRakhi_BP (Game|Player|GetPlayerPawn 0)))
    (Default|TeleporttoBack _asrakhi_bp)))