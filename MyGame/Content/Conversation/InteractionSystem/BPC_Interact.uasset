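; Actor component that lets its owner detect and interact with nearby objects implementing BPI_Interactive.
; On BeginPlay it creates a WBP_Interact widget for prompts.
; Every tick a debug-drawn sphere trace at the owner's location stores the hit interactive actor as HitTarget and shows its LookAtMessage, or clears both when none is found.
; The AI_Interaction input calls InteractWithMessage on a valid target, passing the owner.
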(event Custom|CreateInteractDisplay
  ;[1 1 1] Create interactive display
  (bind _returnvalue (UserInterface|CreateWidget "/Game/Conversation/Inter_UI/WBP_Interact.WBP_Interact_C"))
  (bind _output_get (Variables|Input|SetInteractDisplay _returnvalue))
  (UserInterface|Viewport|AddtoViewport _output_get 0))

(event Input|EnhancedActionEvents|EnhancedInputActionAI_Interaction
  (params (ActionValue :type Boolean) (ElapsedSeconds :type Float%20%28double-precision%29) (TriggeredSeconds :type Float%20%28double-precision%29) (InputAction :type Input%20Action%20Object%20Reference :default "/Game/Conversation/InteractionSystem/AI_Interaction.AI_Interaction"))
  ;[1 1 1] Interaction Input
  (:Started
    (bind _hit_target (Variables|Default|GetHit%20Target)
      (:then
        (Class|BPIInteractive|Interactwith(Message) _hit_target (Components|GetOwner)))
      (:else))))

(event EventBeginPlay
  (CallFunction|CreateInteractDisplay))

(event EventTick
  (params (DeltaSeconds :type Float%20%28single-precision%29))
  (CallFunction|InteractionTrace))

(fn InteractionTrace
  (bind _returnvalue (Components|GetOwner))
  (bind _returnvalue_2 (Transformation|GetActorLocation _returnvalue))
  (bind (_outhit _returnvalue_3) (Collision|SphereTraceByChannel _returnvalue_2 _returnvalue_2 (Variables|Input|GetInteractRadius) "TraceTypeQuery3" false 0 "ForOneFrame"))
  (if _returnvalue_3
    (if (Utilities|DoesObjectImplementInterface (.HitActor (Collision|BreakHitResult _outhit)) "/Game/Conversation/InteractionSystem/BPI_Interactive.BPI_Interactive_C")
      (bind _output_get (Variables|Default|SetHit%20Target (.HitActor (Collision|BreakHitResult _outhit))))
      (bind _interacttext (Class|BPIInteractive|Lookat(Message) _output_get))
      (Default|UpdateInteractText (Variables|Input|GetInteractDisplay) _interacttext)
      (else
        (Variables|Default|SetHit%20Target 0)
        (Default|UpdateInteractText (Variables|Input|GetInteractDisplay))))
    (else
      (Variables|Default|SetHit%20Target 0)
      (Default|UpdateInteractText (Variables|Input|GetInteractDisplay)))))