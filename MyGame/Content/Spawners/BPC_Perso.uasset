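; BPC_Perso is an enemy pawn that chases the player and damages them on contact.
; BeginPlay issues a single AIMoveTo toward the player character, and its vision-range box calls RecibirDaño on any BP_ThirdPersonCharacter that starts overlapping it.
; ReciveDamage lowers its life, updates the health bar widget, and on death awards points directly to the player character before destroying itself.
; A GameState-based score call remains unconnected.
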(event OnComponentBeginOverlap(BoxcoliderRangodeVision)
  (params (OverlappedComponent :type Primitive%20Component%20Object%20Reference) (OtherActor :type Actor%20Object%20Reference) (OtherComp :type Primitive%20Component%20Object%20Reference) (OtherBodyIndex :type Integer) (bFromSweep :type Boolean) (SweepResult :type Hit%20Result%20Structure%20%28by%20ref%29))
  (bind _asbp_third_person_character (Utilities|Casting|CastToBP_ThirdPersonCharacter OtherActor)
    (:then
      (Default|RecibirDaño _asbp_third_person_character 25.0))
    (:CastFailed
      (Development|PrintString "Fallo"))))

(event EventBeginPlay
  (AI|AIMoveTo self "0, 0, 0" (Game|GetPlayerCharacter 0) 0.0 false))

(event Collision|EventActorBeginOverlap
  (params (OtherActor :type Actor%20Object%20Reference)))

(event EventTick
  (params (DeltaSeconds :type Float%20%28single-precision%29)))

(fn ConstructionScript)

(fn ReciveDamage
  (params (DamageTo%20Recive :type Float%20%28double-precision%29))
  (bind _aswbp_health_enemy (Utilities|Casting|CastToWBP_HealthEnemy (UserInterface|GetUserWidgetObject (Variables|Default|GetHealthBar_Widget))))
  (bind _output_get (Variables|Default|SetCurrent%20Life (- (Variables|Default|GetCurrent%20Life) DamageTo%20Recive)))
  (Default|UpdateHealthEnemy _aswbp_health_enemy _output_get (Variables|Default|GetMax%20Life))
  (if (<= _output_get 0.0)
    (bind _asbp_third_person_character (Utilities|Casting|CastToBP_ThirdPersonCharacter (Game|GetPlayerCharacter 0)))
    (Variables|/Game/ThirdPerson/Blueprints/BP_ThirdPersonCharacter.BP_ThirdPersonCharacter_C|SetPuntos%20Totales _asbp_third_person_character (+ (Variables|/Game/ThirdPerson/Blueprints/BP_ThirdPersonCharacter.BP_ThirdPersonCharacter_C|GetPuntos%20Totales _asbp_third_person_character) 100))
    (Actor|DestroyActor)
    (else
      (Development|PrintString "Enemigo recibio daño pero no esta muerto" true true "(R=0.000000,G=0.660000,B=1.000000,A=1.000000)" 5.0))))