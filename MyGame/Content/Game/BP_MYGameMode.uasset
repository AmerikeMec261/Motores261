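; BP_MYGameMode is a game mode that handles scoring by writing to the game state.
; DeadEnemy and ADDScore each cast the current game state to BP_MYGameState and add the given amount to its Score.
; The two functions are identical apart from the parameter name, and the event graph holds only disabled placeholder events.
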(event EventBeginPlay)

(event EventTick
  (params (DeltaSeconds :type Float%20%28single-precision%29)))

(fn ConstructionScript)

(fn DeadEnemy
  (params (EnemyKillScore :type Float%20%28double-precision%29))
  (bind _asbp_mygame_state (Utilities|Casting|CastToBP_MYGameState (Game|GetGameState)))
  (Variables|/Game/Game/BP_MYGameState.BP_MYGameState_C|SetScore _asbp_mygame_state (+ (Variables|/Game/Game/BP_MYGameState.BP_MYGameState_C|GetScore _asbp_mygame_state) EnemyKillScore)))

(fn ADDScore
  (params (Score%20to%20add :type Float%20%28double-precision%29))
  (bind _asbp_mygame_state (Utilities|Casting|CastToBP_MYGameState (Game|GetGameState)))
  (Variables|/Game/Game/BP_MYGameState.BP_MYGameState_C|SetScore _asbp_mygame_state (+ (Variables|/Game/Game/BP_MYGameState.BP_MYGameState_C|GetScore _asbp_mygame_state) Score%20to%20add)))