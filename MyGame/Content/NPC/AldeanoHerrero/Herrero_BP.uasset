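; Blacksmith villager NPC Blueprint holding functions that send the game into and out of a battle arena.
; TeleportToFigth spawns the requested number of Bp_EnemyFight actors once at a fixed point, ignoring TypeOfEnemy, then opens BattleArena_Nieve.
; TeleportToBack opens TrirdPersonMap when no fight enemies remain.
; Rotation, player-location saving and in-map teleport logic are disconnected, and Tick is empty.
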(event Collision|EventActorBeginOverlap
  (params (OtherActor :type Actor%20Object%20Reference)))

(event EventTick
  (params (DeltaSeconds :type Float%20%28single-precision%29))
  ;[1 1 1] Deteccion de Rotación
)

(fn ConstructionScript)

(fn NewFunction)

(fn TeleporttoFigth
  (params (TypeOfEnemy :type Actor%20Object%20Reference) (NumberOfEnemies :type Integer))
  (if (not (Variables|Default|GetSpawnEnemy))
    (Variables|Default|SetSpawnEnemy true)
    (for _index (range 0 NumberOfEnemies)
      ;[1 1 1] Enemy
      (Game|SpawnActorfromClass "/Game/Enemy/Bp_EnemyFight.Bp_EnemyFight_C" (Math|Transform|MakeTransform "-49.999916,-119439.999915,8050.000000" "0, 0, 0" "1.000000,1.000000,1.000000") "AdjustIfPossibleButAlwaysSpawn" "MultiplyWithRoot" 0 0))
    (Game|OpenLevel(byName) "BattleArena_Nieve")))

(fn TeleporttoBack
  (bind _outactors (Actor|GetAllActorsOfClass "/Game/Enemy/Bp_EnemyFight.Bp_EnemyFight_C"))
  (if (<= (Utilities|Array|Length _outactors) 0)
    (Game|OpenLevel(byName) "TrirdPersonMap")))