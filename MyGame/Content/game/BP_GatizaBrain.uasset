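; BP_GatizaBrain holds the collectible-counting and win-condition logic for the game.
; AddCollectible increments the count in the BP_GatizaMemory GameState, fires the AgarrarCollectible dispatcher, then runs WinGame.
; WinGame fires the GanarJuego dispatcher when that count exactly equals CollectiblesToWin.
; Both functions print debug messages; the event graph and construction script are empty.
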(event EventBeginPlay)

(event EventTick
  (params (DeltaSeconds :type Float%20%28single-precision%29)))

(fn ConstructionScript)

(fn AddCollectible
  (bind _asbp_gatiza_memory (Utilities|Casting|CastToBP_GatizaMemory (Game|GetGameState)))
  (Variables|/Game/game/BP_GatizaMemory.BP_GatizaMemory_C|SetNumberCollectible _asbp_gatiza_memory (+ (Variables|/Game/game/BP_GatizaMemory.BP_GatizaMemory_C|GetNumberCollectible _asbp_gatiza_memory) 1))
  (Default|CallAgarrarCollectible)
  (Development|PrintString "agarro collectible")
  (CallFunction|WinGame))

(fn WinGame
  (bind _asbp_gatiza_memory (Utilities|Casting|CastToBP_GatizaMemory (Game|GetGameState)))
  (if (== (Variables|/Game/game/BP_GatizaMemory.BP_GatizaMemory_C|GetCollectiblesToWin _asbp_gatiza_memory) (Variables|/Game/game/BP_GatizaMemory.BP_GatizaMemory_C|GetNumberCollectible _asbp_gatiza_memory))
    (Default|CallGanarJuego)
    (Development|PrintString "Ganaste el juego")))