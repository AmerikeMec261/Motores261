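; BPC_ItemData is an item component that makes its owning actor an inventory pickup.
; On interaction it finds the interactor's BPC_Inventory, passes it the item row name and quantity, and destroys the owner if the pickup succeeds.
; GetItemData looks up the item's row in DT_ItemData, while LookAt currently returns only an empty value.
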(event Custom|Pickup
  (params (Interactor :type Actor%20Object%20Reference))
  (bind _returnvalue (Actor|GetComponentbyClass Interactor "/Game/Inventario/BPC_Inventory.BPC_Inventory_C"))
  (Utilities|IsValid _returnvalue
    (:Is%20Valid
      (bind _success (Default|PickUp _returnvalue (Utilities|Struct|BreakDataTableRowHandle (Variables|Default|GetItemData)) (Variables|Default|GetItemQuantity)))
      (if _success
        (Actor|DestroyActor (Components|GetOwner))))))

(event EventBeginPlay)

(event EventTick
  (params (DeltaSeconds :type Float%20%28single-precision%29)))

(event EventInteractwith
  (params (Interactor :type Actor%20Object%20Reference))
  (CallFunction|Pickup Interactor))

(fn GetItemData
  (bind _returnvalue (Utilities|GetDataTableRow "/Game/Inventario/ItemData/DT_ItemData.DT_ItemData" (.RowName (Utilities|Struct|BreakDataTableRowHandle (Variables|Default|GetItemData))))
    (:then
      (return _returnvalue))))

(fn Lookat
  (return ""))