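; MLK_Brain drives a monster happiness win/lose loop using MonsterHappines in the MLK_Memory game state.
; A one-second timer from BeginPlay re-sets itself and refreshes HUDMENU, without actually decrementing happiness.
; The increase event also only refreshes HUDMENU, mistakenly using happiness plus 50 as the widget array index.
; Victoria and Derrota events print win or loss messages when happiness is near maximum or exactly zero.
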(event Custom|Monster%20happiness
  (CallFunction|IncreaseMonsterHappiness))

(event Custom|VIctoria
  (CallFunction|MonsterHappy))

(event Custom|Derrota
  (CallFunction|MonsterDepressed))

(event Custom|MonsterSadness
  (Utilities|Time|SetTimerbyEvent (delegate Custom|MonsterSadness) 1.0 true)
  (CallFunction|ReduceMonsterHappiness)
  (Development|PrintString "perdió felicidad" true true "(R=0.931383,G=0.081196,B=1.000000,A=1.000000)"))

(event EventBeginPlay
  (Utilities|Time|SetTimerbyEvent (delegate Custom|MonsterSadness) 1.0 true)
  (CallFunction|ReduceMonsterHappiness)
  (Development|PrintString "perdió felicidad" true true "(R=0.931383,G=0.081196,B=1.000000,A=1.000000)"))

(event EventTick
  (params (DeltaSeconds :type Float%20%28single-precision%29)))

(fn ConstructionScript)

(fn ReduceMonsterHappiness
  (bind _asmlk_memory (Utilities|Casting|CastToMLK_Memory (Game|GetGameState)))
  (bind _foundwidgets (Widget|GetAllWidgetsOfClass "/Game/Widgets/HUDMENU.HUDMENU_C" true))
  (bind _ashudmenu (Utilities|Casting|CastToHUDMENU (Utilities|Array|Get(acopy) _foundwidgets)))
  (Default|UpdateMOnsterHappiness _ashudmenu))

(fn MonsterHappy
  (bind _asmlk_memory (Utilities|Casting|CastToMLK_Memory (Game|GetGameState)))
  (if (Math|Float|NearlyEqual(Float) (Variables|/Game/Blueprints/MLK_Memory.MLK_Memory_C|Getmonster%20happines _asmlk_memory) (Variables|/Game/Blueprints/MLK_Memory.MLK_Memory_C|Getmax%20monster%20happiness _asmlk_memory) 0.5)
    (Development|PrintString "¡Ganaste!" true true "(R=0.015126,G=1.000000,B=0.000000,A=1.000000)" 2e+01)))

(fn MonsterDepressed
  (bind _asmlk_memory (Utilities|Casting|CastToMLK_Memory (Game|GetGameState))
    (:then
      (if (== (Variables|/Game/Blueprints/MLK_Memory.MLK_Memory_C|Getmonster%20happines _asmlk_memory) 0.0)
        (Development|PrintString "Perdiste :(")))
    (:CastFailed
      (Development|PrintString "Inmortal Kaiju"))))

(fn IncreaseMonsterHappiness
  (bind _asmlk_memory (Utilities|Casting|CastToMLK_Memory (Game|GetGameState))
    (:then
      (bind _foundwidgets (Widget|GetAllWidgetsOfClass "/Game/Widgets/HUDMENU.HUDMENU_C" true))
      (Default|UpdateMOnsterHappiness (Utilities|Array|Get(acopy) _foundwidgets (Math|Float|Truncate (+ (Variables|/Game/Blueprints/MLK_Memory.MLK_Memory_C|Getmonster%20happines _asmlk_memory) 5e+01)))))
    (:CastFailed
      (Development|PrintString "Falló increase"))))