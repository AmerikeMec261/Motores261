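; Enemy character Blueprint that issues an AI move toward a target on spawn and can be damaged until destroyed.
; BeginPlay calls AIMoveTo once, targeting player controller 0 rather than its pawn.
; Receive Damage subtracts from CurrentLife, updates the enemy healthbar widget and destroys the actor at zero life or below.
; If the healthbar widget cast fails, the damage is not applied.
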(event EventBeginPlay
  (AI|AIMoveTo self "0, 0, 0" (Game|GetPlayerController 0) 5.0 false))

(event Collision|EventActorBeginOverlap
  (params (OtherActor :type Actor%20Object%20Reference)))

(event EventTick
  (params (DeltaSeconds :type Float%20%28single-precision%29)))

(fn ConstructionScript)

(fn ReceiveDamage
  (params (DamageToReceive :type Float%20%28double-precision%29))
  (bind _aswb_enemy_healthbar (Utilities|Casting|CastToWb_EnemyHealthbar (UserInterface|GetUserWidgetObject (Variables|Default|GetEnemyHealthbarWidget))))
  (bind _output_get (Variables|Default|SetCurrentLife (- (Variables|Default|GetCurrentLife) DamageToReceive)))
  (Default|UpdateHealthbar _aswb_enemy_healthbar _output_get (Variables|Default|GetMaxLife))
  (if (<= (Variables|Default|GetCurrentLife) 0.0)
    (Actor|DestroyActor)
    (Development|PrintString "Destroy")))