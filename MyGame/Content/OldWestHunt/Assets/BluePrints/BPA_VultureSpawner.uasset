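; Spawner actor that keeps adding BPPC_BrownV vultures to the level for as long as it runs.
; BeginPlay starts a looping two-second timer through CustomEvent and stores its handle, apparently driving the Aumentador spawn event.
; Each spawn picks a random point inside SpawnBox and a random pitch with zero yaw and roll, adjusting for collisions but always spawning.
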(event Custom|CustomEvent
  (bind _returnvalue (Utilities|Time|SetTimerbyEvent (EventDispatchers|CreateEvent :!event Custom|Aumentador) 2.0 true))
  (Variables|Default|SetNewVar _returnvalue))

(event Custom|Aumentador
  (bind _spawnbox (Variables|Default|GetSpawnBox))
  (Game|SpawnActorfromClass "/Game/OldWestHunt/Assets/BluePrints/BPPC_BrownV.BPPC_BrownV_C" (Math|Transform|MakeTransform (Math|Random|RandomPointinBoundingBox (Transformation|GetWorldLocation _spawnbox) (Components|Box|GetScaledBoxExtent _spawnbox)) (Math|Rotator|MakeRotator 0.0 (Math|Random|RandomFloatinRange 15.0 1e+02) 0.0)) "AdjustIfPossibleButAlwaysSpawn" "MultiplyWithRoot" 0 0))

(event EventBeginPlay
  (CallFunction|CustomEvent))

(event Collision|EventActorBeginOverlap
  (params (OtherActor :type Actor%20Object%20Reference)))

(event EventTick
  (params (DeltaSeconds :type Float%20%28single-precision%29)))

(fn ConstructionScript)