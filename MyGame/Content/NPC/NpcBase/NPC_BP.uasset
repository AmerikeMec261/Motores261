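; Base NPC Blueprint that the player can talk to, showing a "Talk to" prompt with the NPC's name.
; Interaction is forwarded to a dialogue component, and leaving the interaction radius ends the dialogue.
; On BeginPlay it casts its owner to BP_AIController and hands over its behavior tree asset.
; While the Startposition flag is set, Tick spins the actor's yaw at RotationSpeed.
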(event OnComponentEndOverlap(InteractionRadius)
  (params (OverlappedComponent :type Primitive%20Component%20Object%20Reference) (OtherActor :type Actor%20Object%20Reference) (OtherComp :type Primitive%20Component%20Object%20Reference) (OtherBodyIndex :type Integer))
  (Default|EndDialogue (Variables|Default|GetBPC_Dialogue)))

(event EventBeginPlay
  (bind _returnvalue (Components|GetOwner))
  (Development|PrintString (Utilities|GetDisplayName _returnvalue))
  (bind _asbp_aicontroller (Utilities|Casting|CastToBP_AIController _returnvalue))
  (bind _output_get (Variables|/Game/Ai/BP_AIController.BP_AIController_C|SetBTAsset _asbp_aicontroller (Variables|Default|GetBehavorTree))))

(event EventInteractwith
  (params (Interactor :type Actor%20Object%20Reference))
  (Default|Interactwith (Variables|Default|GetBPC_Dialogue) Interactor))

(event EventTick
  (params (DeltaSeconds :type Float%20%28single-precision%29))
  ;[1 1 1] Deteccion de Rotación
  (if (Variables|Default|GetStartposition)
    (bind _output_get (Variables|Default|SetAccumulatedRotation (+ (* DeltaSeconds (Variables|Default|GetRotationSpeed)) (Variables|Default|GetAccumulatedRotation))))
    (Transformation|SetActorRotation (Math|Rotator|MakeRotator 0.0 0.0 _output_get))))

(fn ConstructionScript)

(fn Lookat
  (return (Utilities|Text|FormatText "Talk to {x}" (Variables|Input|GetName))))