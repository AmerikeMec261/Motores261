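; Enemy actor that takes damage, shows its health on a widget bar and is destroyed when life runs out.
; RecieveDamage subtracts from CurrentLife, updates the WPP_EnemyHealth widget, then at zero or below destroys the actor and prints a debug string.
; Movement is a single VInterpTo step toward player 0 on BeginPlay; Tick is empty, so it does not keep following.
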(event EventBeginPlay
  (Transformation|SetActorLocation (Math|Interpolation|VInterpTo (Transformation|GetActorLocation) (Transformation|GetActorLocation (Game|GetPlayerCharacter 0)) (Utilities|Time|GetWorldDeltaSeconds) 5.0) false false))

(event Collision|EventActorBeginOverlap
  (params (OtherActor :type Actor%20Object%20Reference)))

(event EventTick
  (params (DeltaSeconds :type Float%20%28single-precision%29)))

(fn ConstructionScript)

(fn RecieveDamage
  (params (DamageToRecieve :type Float%20%28double-precision%29))
  (bind _aswpp_enemy_health (Utilities|Casting|CastToWPP_EnemyHealth (UserInterface|GetUserWidgetObject (Variables|Default|GetWidget))))
  (bind _output_get (Variables|Default|SetCurrentLife (- (Variables|Default|GetCurrentLife) DamageToRecieve)))
  (Default|UpdateHealthbar _aswpp_enemy_health _output_get (Variables|Default|GetMaxLife))
  (if (<= (Variables|Default|GetCurrentLife) 0.0)
    (Actor|DestroyActor)
    (Development|PrintString "mori")))