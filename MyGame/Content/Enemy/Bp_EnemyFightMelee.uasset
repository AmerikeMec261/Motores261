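; Melee enemy, a PaperZD character that chases the player and attacks on reaching them.
; BeginPlay runs a looping AIMoveTo toward the player, calling Attack on success.
; Attack plays its animation and spawns a BPA_EnemyBulletMelee hit actor, with a DoOnce and delay as cooldown.
; Damage arrives via IReceiveDamage, knocking it backward and updating the healthbar widget; at zero life it destroys itself and calls TeleportToBack on Rakhi_BP.
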(event Custom|Attack
  ;[1 1 1] Ataque Enemigo
  (Utilities|FlowControl|DoOnce false :!label _label
    (:Completed
      (Class|PaperZDAnimInstance|JumptoNode (Variables|/Script/PaperZD.PaperZDAnimationComponent|GetAnimInstance (Variables|/Script/PaperZD.PaperZDCharacter|GetAnimationComponent (Class|PaperZDAnimInstance|GetPaperCharacter (Variables|Default|GetAnimInstance)))) "Attakk" "None")
      (Game|SpawnActorfromClass "/Game/Bullet/BPA_EnemyBulletMelee.BPA_EnemyBulletMelee_C" (Transformation|GetSocketTransform (Variables|Default|GetSpawnBullet) "None" "RTS_World") "AlwaysSpawn" "MultiplyWithRoot" self 2e+01 0)
      (Utilities|FlowControl|Sequence
        (:then_0
          (Utilities|FlowControl|Delay 3.0)
          (Variables|Default|SetCanAttack true)
          (goto _label Reset))
        (:then_1
          (Utilities|FlowControl|Delay 1.0)
          (Class|PaperZDAnimInstance|JumptoNode (Variables|/Script/PaperZD.PaperZDAnimationComponent|GetAnimInstance (Variables|/Script/PaperZD.PaperZDCharacter|GetAnimationComponent (Class|PaperZDAnimInstance|GetPaperCharacter (Variables|Default|GetAnimInstance)))) "BackToIDLE" "None"))))))

(event EventBeginPlay
  ;[1 1 1] Disparar hacia el jugador
  (Variables|Default|SetCanAttack false :!label _label)
  (AI|AIMoveTo self "0, 0, 0" (Game|Player|GetPlayerPawn 0) 1e+01 false
    (:OnSuccess
      (Variables|Default|SetCanAttack true)
      (Utilities|FlowControl|Delay 0.5)
      (Class|PaperZDAnimInstance|JumptoNode (Variables|/Script/PaperZD.PaperZDAnimationComponent|GetAnimInstance (Variables|/Script/PaperZD.PaperZDCharacter|GetAnimationComponent (Class|PaperZDAnimInstance|GetPaperCharacter (Variables|Default|GetAnimInstance)))) "BackToIDLE" "None")
      (if (Variables|Default|GetCanAttack)
        (Variables|Default|SetCanAttack true)
        (CallFunction|Attack)
        (goto _label)))))

(event EventIReceiveDamage
  (params (Damage :type Float%20%28double-precision%29))
  (CallFunction|ReceiveDamage Damage))

(fn ConstructionScript)

(fn ReceiveDamage
  (params (DamageToReceive :type Float%20%28double-precision%29))
  (bind _returnvalue (Transformation|GetActorForwardVector))
  (bind _returnvalue_2 (* _returnvalue -5e+02))
  (Character|LaunchCharacter (Math|Vector|MakeVector (.x _returnvalue_2) (.y _returnvalue_2) (.z _returnvalue_2)) false false)
  (bind _aswb_enemy_healthbar (Utilities|Casting|CastToWb_EnemyHealthbar (UserInterface|GetUserWidgetObject (Variables|Default|GetEnemyHealthbarWidget))))
  (bind _output_get (Variables|Default|SetCurrentLife (- (Variables|Default|GetCurrentLife) DamageToReceive)))
  (Default|UpdateHealthbar _aswb_enemy_healthbar _output_get (Variables|Default|GetMaxLife))
  (if (<= (Variables|Default|GetCurrentLife) 0.0)
    (Actor|DestroyActor)
    (bind _asrakhi_bp (Utilities|Casting|CastToRakhi_BP (Game|Player|GetPlayerPawn 0)))
    (Default|TeleporttoBack _asrakhi_bp)))