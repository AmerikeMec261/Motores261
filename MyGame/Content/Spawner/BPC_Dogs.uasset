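; Dog enemy character that chases the player and is meant to sleep briefly instead of dying.
; BeginPlay binds the sleep dispatcher and starts a looping AIMoveTo chase, gated by CanMove.
; ReciveDamage lowers life, updates the WBP_Enemy health bar, and fires the dispatcher when MaxLife, not CurrentLife, is depleted.
; SleepEnemy halts movement, waits, restores full life without refreshing the bar, then resumes chasing.
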(event Custom|SleepEnemy
  (bind _returnvalue (Game|GetPlayerCharacter 0))
  (bind _self self)
  (Class|NavMovementComponent|StopActiveMovement (Variables|Character|GetCharacterMovement))
  (Variables|Default|SetCan%20Move false)
  (Utilities|FlowControl|Delay 2.0)
  (Variables|Default|SetCurrent%20Life (Variables|Default|GetMax%20Life))
  (Variables|Default|SetCan%20Move true)
  (if (Variables|Default|GetCan%20Move) :!label _label
    (AI|AIMoveTo _self "0, 0, 0" _returnvalue 1.2e+02 false
      (:OnSuccess
        (Utilities|FlowControl|Delay 2.0))
      (:OnFail
        _))
    (if (Variables|Default|GetCan%20Move)
      (AI|AIMoveTo _self "0, 0, 0" _returnvalue 1.2e+02 false
        (:OnSuccess
          (goto _label))
        (:OnFail
          (Utilities|FlowControl|Delay 2.0)
          (goto _label))))))

(event EventBeginPlay
  (bind _returnvalue (Game|GetPlayerCharacter 0))
  (bind _self self)
  (EventDispatchers|BindEventtoSleepEnemyDispatcher (delegate Custom|SleepEnemy))
  (if (Variables|Default|GetCan%20Move) :!label _label
    (AI|AIMoveTo _self "0, 0, 0" _returnvalue 1.2e+02 false
      (:OnSuccess
        _)
      (:OnFail
        (Utilities|FlowControl|Delay 2.0)))
    (if (Variables|Default|GetCan%20Move)
      (AI|AIMoveTo _self "0, 0, 0" _returnvalue 1.2e+02 false
        (:OnSuccess
          (Utilities|FlowControl|Delay 2.0)
          (goto _label))
        (:OnFail
          (goto _label))))))

(event Collision|EventActorBeginOverlap
  (params (OtherActor :type Actor%20Object%20Reference)))

(event EventTick
  (params (DeltaSeconds :type Float%20%28single-precision%29)))

(fn ConstructionScript)

(fn ReciveDamage
  (params (Damage%20to%20Recive :type Float%20%28double-precision%29))
  (bind _aswbp_enemy (Utilities|Casting|CastToWBP_Enemy (UserInterface|GetUserWidgetObject (Variables|Default|GetUpdateHealthBar))))
  (bind _output_get (Variables|Default|SetCurrent%20Life (- (Variables|Default|GetCurrent%20Life) Damage%20to%20Recive)))
  (Default|UpdateHealthBar _aswbp_enemy _output_get (Variables|Default|GetMax%20Life))
  (if (<= (Variables|Default|GetMax%20Life) 0.0)
    (Default|CallSleepEnemyDispatcher)))