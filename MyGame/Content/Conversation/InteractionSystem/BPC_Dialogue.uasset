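; BPC_Dialogue is a component that gives an AI-controlled actor a dialogue the player starts by interacting with it.
; The first interaction creates a dialogue display widget with name and portrait and sets the owner's AI controller to a conversing state with the interactor.
; Later interactions signal speaker-finished on the existing dialogue box.
; EndDialogue removes the widget and returns the AI to idle, while LookAt returns empty text.
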(event Custom|CreateDialogueDisplay
  ;[1 1 1] Create Dialogue Display
  (Variables|Default|GetDialogueDisplay
    (:then
      (Default|CallOnSpeakerFinished (Variables|/Game/Conversation/DialogueUI/WBP_DialogueDisplay.WBP_DialogueDisplay_C|GetDialogueBox (Variables|Default|GetDialogueDisplay))))
    (:else
      (bind _returnvalue (UserInterface|CreateWidget "/Game/Conversation/DialogueUI/WBP_DialogueDisplay.WBP_DialogueDisplay_C" 0 (Variables|Input|GetName) (Variables|Input|GetPortrait)))
      (bind _output_get (Variables|Default|SetDialogueDisplay _returnvalue))
      (UserInterface|Viewport|AddtoViewport _output_get 0)
      (bind __aicontroller (Variables|Default|Get%20AIController)
        (:then
          (Default|SetStateasConversating __aicontroller (Variables|Default|GetInteractor)))
        (:else)))))

(event Custom|EndDialogue
  ;[1 1 1] End Dialogue Logic
  (bind _dialoguedisplay (Variables|Default|GetDialogueDisplay)
    (:then
      (Widget|RemovefromParent _dialoguedisplay)
      (Variables|Default|SetDialogueDisplay 0)
      (bind __aicontroller (Variables|Default|Get%20AIController)
        (:then
          (Default|SetStateasIdle __aicontroller))
        (:else)))
    (:else)))

(event EventBeginPlay
  ;[1 1 1] Set reference to AI controller
  (bind _asbp_aicontroller (Utilities|Casting|CastToBP_AIController (AI|GetAIController (Components|GetOwner))))
  (Variables|Default|Set%20AIController _asbp_aicontroller))

(event EventInteractwith
  (params (Interactor :type Actor%20Object%20Reference))
  (Variables|Default|SetInteractor Interactor)
  (CallFunction|CreateDialogueDisplay))

(fn Lookat
  (return ""))